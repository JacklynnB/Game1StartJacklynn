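; Patrolling enemy AI that walks between control points, chases the player on sight and sends them back to a checkpoint on contact.
; BeginPlay gathers tagged points and randomizes walk speed; a recursive AIMoveTo loop visits them, reshuffling after each lap.
; PawnSensing starts a periodically reissued move toward the player, with no effective reset of PlayerSeen.
; Sphere overlap plays a crunch, loads the checkpoint and resumes patrol; breathing-sound logic is disconnected.
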(event `self.ReceiveBeginPlay`
  ;[1 1 1] Initialize and Walking Speed
  (bind _outactors (`GameplayStatics.GetAllActorsOfClassWithTag` "/Script/Engine.Actor" "ControlTestPoint1"))
  (`KismetSystemLibrary.PrintString` (`KismetStringLibrary.Concat_StrStr` "There Are" (`KismetStringLibrary.Conv_IntToString` (`KismetArrayLibrary.Array_Length` _outactors)) "Control Points"))
  (`KismetArrayLibrary.Array_Shuffle` _outactors)
  (set `CharacterMovementComponent.MaxWalkSpeed` (`KismetMathLibrary.Conv_IntToDouble` (* (`KismetMathLibrary.RandomIntegerInRange` 4 8) 25)) (`self.CharacterMovement`))
  (`self.GoToCTP`))

(event `GoToCTP`
  ;[1 1 1] Patrol Control Points
  (`|AIMoveTo` self (`self.K2_GetActorLocation` (`|GetArrayItem` (stale `self.ReceiveBeginPlay` _outactors) (`self.CurrentCTP`))) null 200.0 ; Move ourselves to the players location by const updating and stopping 2 meters away
    (:`OnSuccess`
      (`KismetSystemLibrary.PrintString` "Patrol'd"))
    (:`OnFail`
      (`KismetSystemLibrary.PrintString` "gooby")))
  (bind _result (`/Engine/EditorBlueprintResources/StandardMacros.IncrementInt` (`self.CurrentCTP`))
    (:`  `
      (if (>= _result (`KismetArrayLibrary.Array_Length` (stale `self.ReceiveBeginPlay` _outactors)))
        (set `self.CurrentCTP` 0)
        (`KismetArrayLibrary.Array_Shuffle` (stale `self.ReceiveBeginPlay` _outactors)))
      (`KismetSystemLibrary.Delay` 1.0)
      (`self.GoToCTP`))))

(event `GoToPlayer`
  (if (`self.PlayerSeen`)
    (`|AIMoveTo` self (0.0 0.0 0.0) (`GameplayStatics.GetPlayerCharacter` 0)
      (:`then`
        (`KismetSystemLibrary.Delay` 10.0)
        (`self.GoToPlayer`)))
    (else
      (set `self.PlayerSeen` false))))

(event `self.Sphere.OnComponentBeginOverlap`
  (params (OverlappedComponent :type "PrimitiveComponent Object Reference") (OtherActor :type "Actor Object Reference") (OtherComp :type "PrimitiveComponent Object Reference") (OtherBodyIndex :type Integer) (bFromSweep :type Boolean) (SweepResult :type "HitResult Structure (by ref)"))
  ;[1 1 1] Kill Player
  (bind _asbp_third_person_character_custom (cast `/Game/Blueprints/BP_ThirdPersonCharacterCustom` OtherActor))
  (`GameplayStatics.PlaySound2D` "/Game/Audio/Crunch.Crunch" 1.0 1.0 0.0 null null)
  (`/Game/Blueprints/BP_ThirdPersonCharacterCustom.Load Checkpoint` _asbp_third_person_character_custom)
  (`self.GoToCTP`))

(event `self.ReceiveTick`
  (params (DeltaSeconds :type "Float (single-precision)")))

(event `self.PawnSensing.OnSeePawn`
  (params (Pawn :type "Pawn Object Reference"))
  (set `self.PlayerSeen` true)
  (`self.GoToPlayer`))

(fn `UserConstructionScript`)